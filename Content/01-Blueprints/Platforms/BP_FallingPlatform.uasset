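; BP_FallingPlatform is a platform that falls shortly after the player steps on it and then respawns.
; On BeginPlay it stores its transform.
; When a BP_Player overlaps its Box, it waits briefly, enables physics on the Cube, and after a few seconds disables it.
; It then spawns a fresh copy at the stored location and rotation and destroys itself, resetting by replacement.
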(event `self.ReceiveBeginPlay`
  (set `self.DefaultTransform` (`self.GetTransform`)))

(event `self.Box.OnComponentBeginOverlap`
  (params (OverlappedComponent :type "PrimitiveComponent Object Reference") (OtherActor :type "Actor Object Reference") (OtherComp :type "PrimitiveComponent Object Reference") (OtherBodyIndex :type Integer) (bFromSweep :type Boolean) (SweepResult :type "HitResult Structure (by ref)"))
  (bind (_defaulttransform_location _defaulttransform_rotation) (`KismetMathLibrary.BreakTransform` (`self.DefaultTransform`)))
  (cast `/Game/01-Blueprints/Player/BP_Player` OtherActor)
  (`KismetSystemLibrary.Delay` 1.0)
  (`PrimitiveComponent.SetSimulatePhysics` (`self.Cube`) true)
  (`KismetSystemLibrary.Delay` 5.0)
  (`PrimitiveComponent.SetSimulatePhysics` (`self.Cube`) false)
  (`|SpawnActorFromClass` "BP_FallingPlatform_C" (`KismetMathLibrary.MakeTransform` _defaulttransform_location _defaulttransform_rotation) "AlwaysSpawn" "MultiplyWithRoot" null null)
  (`self.K2_DestroyActor`))

(fn `UserConstructionScript`)