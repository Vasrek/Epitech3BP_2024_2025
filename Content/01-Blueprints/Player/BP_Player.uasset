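; BP_Player is the playable character, handling movement, look, jumping, score and respawning.
; On BeginPlay it adds the Enhanced Input mapping context, saves its starting transform as the respawn point and creates the WBP_HUD widget.
; Move input follows control yaw.
; RespawnPlayer teleports back to that point and applies a score penalty through AddScore, which clamps the score at zero and updates the HUD.
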(event `self.ReceiveBeginPlay`
  (bind _returnvalue (`GameplayStatics.GetPlayerController` 0))
  (bind _returnvalue_2 (pcsubsystem `EnhancedInputLocalPlayerSubsystem` (`GameplayStatics.GetPlayerController` 0)))
  (`/Engine/EditorBlueprintResources/StandardMacros.IsValid` _returnvalue_2
    (:`Is Valid`
      (`EnhancedInputSubsystemInterface.AddMappingContext` _returnvalue_2 "/Game/01-Blueprints/Inputs/IMC_Player.IMC_Player" 0 (struct))
      (set `self.RespawnTransform` (`self.GetTransform`))
      (bind _returnvalue_3 (`|CreateWidget` "/Game/01-Blueprints/Widgets/WBP_HUD.WBP_HUD_C"))
      (bind _output_get (set `self.HUDRef` _returnvalue_3))
      (`UserWidget.AddToViewport` _output_get 0)
      (`/Game/01-Blueprints/Widgets/WBP_HUD.UpdateTextScore` _output_get 0)
      (`WidgetBlueprintLibrary.SetInputMode_GameOnly` _returnvalue)
      (set `PlayerController.bShowMouseCursor` false _returnvalue))))

(event `EnhancedInput|/Game/01-Blueprints/Inputs/Actions/IA_Player_Move`
  (params (ActionValue :type "Vector2D Structure") (ElapsedSeconds :type "Float (double-precision)") (TriggeredSeconds :type "Float (double-precision)") (InputAction :type "InputAction Object Reference" :default "/Game/01-Blueprints/Inputs/Actions/IA_Player_Move.IA_Player_Move"))
  (bind (_returnvalue_roll _returnvalue_pitch _returnvalue_yaw) (`KismetMathLibrary.BreakRotator` (`self.GetControlRotation`)))
  (bind (_returnvalue_roll_2 _returnvalue_pitch_2 _returnvalue_yaw_2) (`KismetMathLibrary.BreakRotator` (`self.GetControlRotation`)))
  (:`Triggered`
    (`self.AddMovementInput` (`KismetMathLibrary.GetForwardVector` (`KismetMathLibrary.MakeRotator` 0.0 0.0 _returnvalue_yaw)) ActionValue_Y)
    (`self.AddMovementInput` (`KismetMathLibrary.GetRightVector` (`KismetMathLibrary.MakeRotator` 0.0 0.0 _returnvalue_yaw_2)) ActionValue_X)))

(event `EnhancedInput|/Game/01-Blueprints/Inputs/Actions/IA_Player_Look`
  (params (ActionValue :type "Vector2D Structure") (ElapsedSeconds :type "Float (double-precision)") (TriggeredSeconds :type "Float (double-precision)") (InputAction :type "InputAction Object Reference" :default "/Game/01-Blueprints/Inputs/Actions/IA_Player_Look.IA_Player_Look"))
  (:`Triggered`
    (`self.AddControllerYawInput` ActionValue_X)
    (`self.AddControllerPitchInput` ActionValue_Y)))

(event `EnhancedInput|/Game/01-Blueprints/Inputs/Actions/IA_Player_Jump`
  (params (ActionValue :type Boolean) (ElapsedSeconds :type "Float (double-precision)") (TriggeredSeconds :type "Float (double-precision)") (InputAction :type "InputAction Object Reference" :default "/Game/01-Blueprints/Inputs/Actions/IA_Player_Jump.IA_Player_Jump"))
  (:`Started`
    (`self.Jump`))
  (:`Completed`
    (`self.StopJumping`)))

(event `RespawnPlayer`
  (`self.K2_SetActorTransform` (`self.RespawnTransform`) false true)
  (`self.AddScore` -5)
  (`/Game/01-Blueprints/Widgets/WBP_HUD.UpdateTextScore` (`self.HUDRef`) (`self.CurrentScore`)))

(event `AddScore`
  (params (ScoreToAdd :type Integer))
  (bind _output_get (set `self.CurrentScore` (+ ScoreToAdd (`self.CurrentScore`))))
  (if (<= _output_get 0)
    (set `self.CurrentScore` 0))
  (`/Game/01-Blueprints/Widgets/WBP_HUD.UpdateTextScore` (`self.HUDRef`) (`self.CurrentScore`)))

(fn `UserConstructionScript`)